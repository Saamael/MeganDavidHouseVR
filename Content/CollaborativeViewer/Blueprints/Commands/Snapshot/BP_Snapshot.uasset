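; Snapshot command for the Collaborative Viewer, adding a "Take" option that captures from a photo frame when no HMD is enabled.
; Enabling it narrows pawn collision queries and replaces existing BP_Photo actors with one at the camera, scaled to world scale.
; Left press hands the frame to the pawn's transform component for left- or right-hand manipulation.
; Disabling restores collision and field of view, stops transforming and destroys the frame.
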(event Custom|Enabled
  (bind _basepawn (Variables|Default|GetBasePawn))
  ;[0.3384 0.6313 1] Setup Option Buttons
  (Variables|Default|SetActivated true)
  (Variables|/Game/CollaborativeViewer/Blueprints/Pawn/BP_BasePawn.BP_BasePawn_C|SetCollisionType _basepawn (Utilities|Array|MakeArray "ObjectTypeQuery9"))
  (Utilities|IsValid _basepawn
    (:Is%20Valid
      (CallFunction|Setup))))

(event Custom|Setup
  (bind _basepawn (Variables|Default|GetBasePawn))
  (bind _camera (Variables|/Game/CollaborativeViewer/Blueprints/Pawn/BP_BasePawn.BP_BasePawn_C|GetCamera _basepawn))
  (bind _returnvalue (Transformation|GetWorldTransform _camera))
  ;[1 1 1] Set photo Frame Location
  (Variables|Default|SetPhotoTransform (Math|Transform|MakeTransform (.location _returnvalue) (.rotation _returnvalue) (Math|Conversions|ToVector(Float) (Variables|/Game/CollaborativeViewer/Blueprints/Pawn/BP_BasePawn.BP_BasePawn_C|GetCurrentWorldScale _basepawn))))
  ;[1 1 1] Delete previous BP Photo
  (bind _outactors (Actor|GetAllActorsOfClass "/Game/CollaborativeViewer/Blueprints/Commands/Snapshot/BPs/BP_Photo.BP_Photo_C"))
  (Actor|DestroyActor _outactors)
  ;[1 1 1] Create new BP Photo
  (bind _returnvalue_2 (Game|SpawnActorfromClass "/Game/CollaborativeViewer/Blueprints/Commands/Snapshot/BPs/BP_Photo.BP_Photo_C" (Variables|Default|GetPhotoTransform) "Undefined" 0 0))
  (Default|Init _returnvalue_2)
  (Variables|Default|SetCurrentPhotoFrame _returnvalue_2))

(event Custom|Bind_Options
  (bind _optionsbuttons (Variables|Default|GetOptionsButtons))
  (bind _output (Utilities|Array|Get(acopy) _optionsbuttons))
  (bind _asoption_button (Utilities|Casting|CastToOption_Button _output))
  ;[0.3384 0.6313 1] Setup Option Buttons
  (Variables|/Game/CollaborativeViewer/UMG/GameMenu/Option_Button.Option_Button_C|SetWhenExecute _asoption_button "NewEnumerator0")
  (EventDispatchers|BindEventtoExecute _asoption_button (delegate Custom|Option1))
  (EventDispatchers|BindEventtoEnabled _asoption_button (delegate Custom|Enabled))
  (EventDispatchers|BindEventtoDisabled _asoption_button (delegate Custom|OnDisable))
  (Game|AssignOnDestroyed (Game|Player|GetPlayerPawn 0) (delegate Custom|OnDestroyed)))

(event Custom|OnDisable
  (bind _returnvalue (Game|Player|GetPlayerPawn 0))
  (bind _currentphotoframe (Variables|Default|GetCurrentPhotoFrame))
  (bind _basepawn (Variables|Default|GetBasePawn))
  (bind _returnvalue_2 (Actor|GetComponentbyClass _returnvalue "/Game/CollaborativeViewer/Blueprints/Commands/Transform/BP_TransformComponent.BP_TransformComponent_C"))
  ;[0.3384 0.6313 1] Setup Option Buttons
  (Variables|Default|SetActivated false)
  (Variables|/Game/CollaborativeViewer/Blueprints/Pawn/BP_BasePawn.BP_BasePawn_C|SetCollisionType _basepawn (Utilities|Array|MakeArray "ObjectTypeQuery1" "ObjectTypeQuery2"))
  (Variables|/Script/Engine.CameraComponent|SetFieldOfView (Variables|/Game/CollaborativeViewer/Blueprints/Pawn/BP_BasePawn.BP_BasePawn_C|GetCamera _basepawn) 9e+01)
  (Utilities|IsValid _returnvalue
    (:Is%20Valid
      (Default|SetupTransformComponent _returnvalue_2 false false false false)
      (Variables|/Game/CollaborativeViewer/Blueprints/Commands/Transform/BP_TransformComponent.BP_TransformComponent_C|SetIs_L_Updating _returnvalue_2 false)
      (Variables|/Game/CollaborativeViewer/Blueprints/Commands/Transform/BP_TransformComponent.BP_TransformComponent_C|SetIs_R_Updating _returnvalue_2 false)
      (Utilities|IsValid _currentphotoframe
        (:Is%20Valid
          (Actor|DestroyActor _currentphotoframe))))))

(event Custom|Option1
  (params (id :type Integer) (Actor :type Actor%20Object%20Reference) (IsRightHand :type Boolean))
  ;[0.3384 0.6313 1] Setup Option Buttons
  (if (not (Class|HeadMountedDisplayFunctionLibrary|IsHeadMountedDisplayEnabled))
    (Default|DoCapture (Variables|Default|GetCurrentPhotoFrame))))

(event Custom|LeftMousePressed
  (params (Actor :type Actor%20Object%20Reference) (RightHand :type Boolean))
  (bind _basepawn (Variables|Default|GetBasePawn))
  (bind _returnvalue (Actor|GetComponentbyClass _basepawn "/Game/CollaborativeViewer/Blueprints/Commands/Transform/BP_TransformComponent.BP_TransformComponent_C"))
  ;[0 1 0.1488] BeginPlay
  ;;[1 1 1] Binding Button
  (if (Variables|Default|GetActivated)
    (Default|SetStartTransform (Actor|GetComponentbyClass (Variables|Default|GetBasePawn) "/Game/CollaborativeViewer/Blueprints/Commands/Transform/BP_TransformComponent.BP_TransformComponent_C") (Variables|Default|GetCurrentPhotoFrame) RightHand)
    (Default|SetupTransformComponent _returnvalue false true false false)
    (if RightHand
      (Variables|/Game/CollaborativeViewer/Blueprints/Commands/Transform/BP_TransformComponent.BP_TransformComponent_C|SetIs_R_Updating _returnvalue true)
      (else
        (Variables|/Game/CollaborativeViewer/Blueprints/Commands/Transform/BP_TransformComponent.BP_TransformComponent_C|SetIs_L_Updating _returnvalue true)))))

(event Custom|OnDestroyed
  (params (DestroyedActor :type Actor%20Object%20Reference))
  (bind _currentphotoframe (Variables|Default|GetCurrentPhotoFrame))
  ;[0.3384 0.6313 1] Setup Option Buttons
  (Utilities|IsValid _currentphotoframe
    (:Is%20Valid
      (Actor|DestroyActor _currentphotoframe))))

(event EventExecuteAfterSpawnPawn
  ;[0 1 0.1488] BeginPlay
  (Variables|Default|SetIcon "/Game/CollaborativeViewer/Blueprints/Commands/Snapshot/IconSnapshot.IconSnapshot")
  (Variables|Default|SetOptionsButtonNames (Utilities|Array|MakeArray "Take"))
  (Variables|Default|SetName "Snapshot")
  (CallFunction|SetVariables)
  (CallFunction|CreateContextualButon)
  (CallFunction|BindOptions)
  (EventDispatchers|BindEventtoMouseLeftPressed (Variables|Default|GetBasePawn) (delegate Custom|LeftMousePressed)))